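; Bunny pawn that moves to a destination passed to Goto, then plays a timed animation before accepting another move.
; Tick interpolates location and rotation, with speed chosen by distance and pushed to bunny_anim_bp.
; After stopping and turning back to zero rotation, it picks a random DurDict key.
; That key sets how long Anim_Attack plays before the mesh returns to Animation Blueprint mode and InAction clears.
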(event `self.ReceiveBeginPlay`)

(event `self.ReceiveTick`
  (params (DeltaSeconds :type "Float (single-precision)"))
  (bind _bunny_mesh (`self.bunny_mesh`))
  (bind (_value _returnvalue) (`BlueprintMapLibrary.Map_Find` (`self.dur_dict`) (`self.anim_to_play`)))
  (`self.set_location` DeltaSeconds)
  (`self.set_rotation` DeltaSeconds)
  (if _returnvalue
    (`/Engine/EditorBlueprintResources/StandardMacros.DoOnce` false :!label _label
      (:`Completed`
        (`SkeletalMeshComponent.PlayAnimation` _bunny_mesh "/Game/Bunny/Animations/Anim_Attack.Anim_Attack" false)
        (`KismetSystemLibrary.Delay` _value)
        (`SkeletalMeshComponent.SetAnimationMode` _bunny_mesh "AnimationBlueprint")
        (set `self.anim_to_play` 0)
        (set `self.in_action` false)
        (goto _label :!via `Reset`)))))

(fn `goto`
  (params (destination :type "Vector Structure"))
  (if (not (`self.in_action`))
    (set `self.in_action` true)
    (set `self.in_move` true)
    (set `self.destination` destination)
    (bind _asbunny_anim_bp (cast `/Game/BP/anim/bunny_anim_bp` (`SkeletalMeshComponent.GetAnimInstance` (`self.bunny_mesh`))))
    (if (> (`KismetMathLibrary.VSize` (- (`self.K2_GetActorLocation`) destination)) 200.0)
      (bind _output_get (set `self.speed` 100.0))
      (set `/Game/BP/anim/bunny_anim_bp.speed` _output_get _asbunny_anim_bp)
      (else
        (bind _output_get_2 (set `self.speed` 50.0))
        (set `/Game/BP/anim/bunny_anim_bp.speed` _output_get_2 _asbunny_anim_bp)))))

(fn `set_location`
  (params (delta :type "Float (double-precision)"))
  (bind _returnvalue (`self.K2_GetActorLocation`))
  (bind _returnvalue_2 (`KismetMathLibrary.VInterpTo_Constant` _returnvalue (`self.destination`) delta (`self.speed`)))
  (if (`self.in_move`)
    (`self.K2_SetActorLocation` _returnvalue_2)
    (if (== _returnvalue _returnvalue_2)
      (`self.stop_move`))))

(fn `set_rotation`
  (params (delta :type "Float (double-precision)"))
  (bind _returnvalue (`self.K2_GetActorRotation`))
  (bind _rspeed (`self.rspeed`))
  (bind (_returnvalue_x _returnvalue_y) (`KismetMathLibrary.BreakVector` (- (`self.destination`) (`self.K2_GetActorLocation`))))
  (bind (_returnvalue_roll _returnvalue_pitch _returnvalue_yaw) (`KismetMathLibrary.BreakRotator` (`KismetMathLibrary.Conv_VectorToRotator` (`KismetMathLibrary.MakeVector` 0.0 _returnvalue_y))))
  (if (`self.in_move`)
    (`self.K2_SetActorRotation` (`KismetMathLibrary.RInterpTo_Constant` (`self.K2_GetActorRotation`) (`KismetMathLibrary.MakeRotator` 0.0 0.0 (* -1 _returnvalue_yaw)) delta _rspeed))
    (set `self.in_rotation` true)
    (elif (== _returnvalue (struct))
      (if (`self.in_rotation`)
        (set `self.in_rotation` false)
        (set `self.anim_to_play` (`KismetMathLibrary.RandomIntegerInRange` 1 (`BlueprintMapLibrary.Map_Length` (`self.dur_dict`))))
        (bind _asbunny_anim_bp (cast `/Game/BP/anim/bunny_anim_bp` (`SkeletalMeshComponent.GetAnimInstance` (`self.bunny_mesh`))))
        (set `/Game/BP/anim/bunny_anim_bp.is_anim` true _asbunny_anim_bp))
      (else
        (`self.K2_SetActorRotation` (`KismetMathLibrary.RInterpTo_Constant` _returnvalue (struct) delta _rspeed))
        (set `self.in_rotation` true)))))

(fn `stop_move`
  (set `self.in_move` false)
  (bind _output_get (set `self.speed` 0.0))
  (bind _asbunny_anim_bp (cast `/Game/BP/anim/bunny_anim_bp` (`SkeletalMeshComponent.GetAnimInstance` (`self.bunny_mesh`))))
  (set `/Game/BP/anim/bunny_anim_bp.speed` _output_get _asbunny_anim_bp))

(fn `UserConstructionScript`)